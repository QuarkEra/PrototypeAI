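; BP_PowerLines is an environment tool that lays copies of a chosen mesh along a spline, by its name for power lines.
; The construction script derives spacing from the mesh's X bounds plus Offset, then fits the instance count to the spline length.
; Each copy is an Instanced Static Mesh instance at unit scale, aimed at the next sampled point rather than bent along the curve.
; The event graph has no active logic.
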(fn `Get LocationAtIndex`
  (params (A :type "Float (double-precision)"))
  (returns (ReturnValue :type "Vector Structure"))
  (return (`SplineComponent.GetLocationAtDistanceAlongSpline` (`self.Spline`) (* A (`self.Spacing`)) "Local")))

(fn `UserConstructionScript`
  (bind (_min _max) (break `Box` (`StaticMesh.GetBoundingBox` (`self.PlacedMesh`))))
  (`StaticMeshComponent.SetStaticMesh` (`self.InstancedStaticMesh`) (`self.PlacedMesh`))
  (bind _output_get (set `self.Spacing` (+ (.x (- _max _min)) (`self.Offset`))))
  (bind _output_get_2 (set `self.NumInstances` (`KismetMathLibrary.FFloor` (/ (`SplineComponent.GetSplineLength` (`self.Spline`)) _output_get))))
  (for _index (range (+ _output_get_2 1))
    (bind _returnvalue (`self.Get LocationAtIndex` (`KismetMathLibrary.Conv_IntToDouble` _index)))
    (`InstancedStaticMeshComponent.AddInstance` (`self.InstancedStaticMesh`) (`KismetMathLibrary.MakeTransform` _returnvalue (`KismetMathLibrary.MakeRotFromX` (- (`self.Get LocationAtIndex` (`KismetMathLibrary.Conv_IntToDouble` (+ _index 1))) _returnvalue))) false)))