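; BP_InteractBackDoorDirty is an interactable door that swings open and closed on alternating Interact calls.
; Interact finds an actor of the passed class and toggles the IsClosed flag.
; On opening, a dot product between the door's forward vector and the direction from that actor picks the swing sign.
; A timeline lerps the Door's yaw up to 90 degrees either way, and plays in reverse to close.
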(event `self.Interact`
  (params (InteractingActorClass :type "Actor Class Reference"))
  (if (`KismetSystemLibrary.IsValidClass` InteractingActorClass)
    (bind _returnvalue (`GameplayStatics.GetActorOfClass` InteractingActorClass))
    (if (`self.bIsClosed`)
      (set `self.bIsClosed` false)
      (set `self.DotProduct` (`KismetMathLibrary.Dot_VectorVector` (`KismetMathLibrary.Normal` (- (`self.K2_GetActorLocation` self) (`self.K2_GetActorLocation` _returnvalue))) (`self.GetActorForwardVector`)))
      (bind (_direction _rotation) (`Timeline|Timeline` :!via `PlayFromStart` :!label _label)
        (:`Update`
          (bind (_returnvalue_roll _returnvalue_pitch _returnvalue_yaw) (`KismetMathLibrary.BreakRotator` (`KismetMathLibrary.MakeRotator` 0.0 0.0 (`KismetMathLibrary.Lerp` 0.0 (`KismetMathLibrary.SelectFloat` -90.0 90.0 (>= (`self.DotProduct`) 0.0)) _rotation))))
          (`SceneComponent.K2_SetRelativeRotation` (`self.Door`) (`KismetMathLibrary.MakeRotator` 0.0 0.0 _returnvalue_yaw) false false)))
      (else
        (set `self.bIsClosed` true)
        (goto _label :!via `ReverseFromEnd`)))))

(fn `UserConstructionScript`)