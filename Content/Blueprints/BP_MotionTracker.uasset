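; Motion tracker that audibly warns the player when the BP_Alien is moving nearby.
; BeginPlay caches the alien and starts Beep, a self-rescheduling timer that plays a 2D radar pulse only while the alien has velocity and is within FarDistance of the player.
; Pitch rises as the distance shrinks, and UpdateTimerByDistance maps that distance to the next interval between TimeMin and TimeMax, so no Tick logic is used.
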(event `self.ReceiveBeginPlay`
  (bind _returnvalue (`GameplayStatics.GetActorOfClass` "/Game/Characters/BP_Alien.BP_Alien_C"))
  (set `self.Alien` _returnvalue)
  (`KismetSystemLibrary.K2_SetTimer` null "Beep" (`self.Time`)))

(event `self.ReceiveTick`
  (params (DeltaSeconds :type "Float (single-precision)")))

(fn `Beep`
  (bind _returnvalue (`KismetMathLibrary.Vector_Distance` (`self.K2_GetActorLocation` (`GameplayStatics.GetPlayerCharacter` 0)) (`self.K2_GetActorLocation` (`self.Alien`))))
  (bind _returnvalue_2 (`KismetMathLibrary.FClamp` (+ (* (/ _returnvalue (`self.CloseDistance`)) -1.0) (`self.PitchMax`)) (`self.PitchMin`) (`self.PitchMax`)))
  (`KismetSystemLibrary.K2_ClearTimer` null "Beep")
  (if (> (`KismetMathLibrary.VSize` (`self.GetVelocity` (`self.Alien`))) 0.0)
    (if (< _returnvalue (`self.FarDistance`))
      (bind _output_get (set `self.Pitch Multiplier` _returnvalue_2))
      (`GameplayStatics.SpawnSound2D` "/Game/Audio/MotionTracker/449672__matrixxx__radar-something-detected-one-pulse_Cue.449672__matrixxx__radar-something-detected-one-pulse_Cue" 1.5 _output_get 0.0 null)
      (else
        (set `self.Pitch Multiplier` _returnvalue_2 :!label _label)))
    (else
      (goto _label)))
  (`self.UpdateTimerByDistance`))

(fn `UpdateTimerByDistance`
  (set `self.Time` (`KismetMathLibrary.MapRangeClamped` (`KismetMathLibrary.Vector_Distance` (`self.K2_GetActorLocation` (`GameplayStatics.GetPlayerCharacter` 0)) (`self.K2_GetActorLocation` (`self.Alien`))) 0.0 (`KismetMathLibrary.Conv_IntToDouble` (`self.FarDistance`)) (`self.TimeMin`) (`self.TimeMax`)))
  (`KismetSystemLibrary.K2_SetTimer` null "Beep" (`self.Time`)))

(fn `UserConstructionScript`)