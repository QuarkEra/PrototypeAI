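; BP_Flare is a flare actor that lights up on spawn and acts as an audible distraction for AI.
; BeginPlay starts particles, audio and capsule, toggles the point light, and runs a looping timer that reports long-range noise at the flare's location.
; After Duration, it clears the timer, stops audio and particles, and toggles the light again.
; The construction script registers its perception stimuli source for hearing.
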(event `self.Capsule.OnComponentActivated`
  (params (Component :type "ActorComponent Object Reference") (bReset :type Boolean))
  ;[1 1 1] It didnt activate automatically
)

(event `self.ReceiveBeginPlay`
  (`ActorComponent.Activate` (`self.Capsule`) false)
  (`SceneComponent.ToggleVisibility` (`self.PointLight`) false)
  (`AudioComponent.Play` (`self.Audio`) 0.0)
  (`ActorComponent.Activate` (`self.ParticleSystem1`) false)
  (`ActorComponent.Activate` (`self.ParticleSystem`) false)
  (`|ExecutionSequence`
    (:`then_0`
      (`KismetSystemLibrary.K2_SetTimer` null "Make Noise for Distraction" 0.2 true))
    (:`then_1`
      (`KismetSystemLibrary.Delay` (`self.Duration`))
      (`KismetSystemLibrary.K2_ClearTimer` null "Make Noise for Distraction")
      (`AudioComponent.Stop` (`self.Audio`))
      (`ActorComponent.Deactivate` (`self.ParticleSystem1`))
      (`ActorComponent.Deactivate` (`self.ParticleSystem`))
      (`SceneComponent.ToggleVisibility` (`self.PointLight`) false))))

(fn `Make Noise for Distraction`
  (`AISense_Hearing.ReportNoiseEvent` (`self.K2_GetActorLocation` self) 1.0 (`self.GetInstigator` self) 20000.0 "Default__AISense_Hearing")
  (return))

(fn `UserConstructionScript`
  (bind _aiperceptionstimulisource (`self.AIPerceptionStimuliSource`))
  (`AIPerceptionStimuliSourceComponent.RegisterForSense` _aiperceptionstimulisource "/Script/AIModule.AISense_Hearing")
  (`AIPerceptionStimuliSourceComponent.RegisterWithPerceptionSystem` _aiperceptionstimulisource))