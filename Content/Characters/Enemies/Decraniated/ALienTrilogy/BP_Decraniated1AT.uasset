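; BP_Decraniated1AT is a Decraniated enemy, in the Alien Trilogy folder, that can open closed doors in its path.
; On BeginPlay it starts a looping timer that periodically runs CheckForDoorsToOpen.
; That function line-traces a short distance forward on the Visibility channel and, on hitting a closed BP_InteractDoor, sends it InteractMessage with MonsterCharacter.
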(event `self.ReceiveBeginPlay`
  (`KismetSystemLibrary.K2_SetTimer` null "CheckForDoorsToOpen" 1.5 true))

(fn `CheckForDoorsToOpen`
  (bind _returnvalue (`self.K2_GetActorLocation`))
  (bind _outhit (`KismetSystemLibrary.LineTraceSingle` _returnvalue (+ _returnvalue (* (`self.GetActorForwardVector`) 100.0)) "TraceTypeQuery1"))
  (bind _asbp_interact_door (cast `/Game/Environment/Doors/BP_InteractDoor` (`.HitActor` (`GameplayStatics.BreakHitResult` _outhit))))
  (if (`/Game/Environment/Doors/BP_InteractDoor.bIsClosed` _asbp_interact_door)
    (message `/Game/Blueprints/Interfaces/BPI_Interact.Interact` _asbp_interact_door "/Script/GunsOfDinosaurs.MonsterCharacter")))

(fn `UserConstructionScript`)