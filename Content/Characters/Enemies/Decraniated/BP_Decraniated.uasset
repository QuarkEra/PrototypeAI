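; Decraniated enemy character that opens doors in its path and shows a movement-dependent blip, intended for a motion tracker.
; A looping timer runs a short forward line trace and sends an interact message to any BP_InteractDoor hit.
; Tick zeroes the sprite's scale when stationary; while moving, it remaps ScaleSprite using max walk speed as the output bound, rather than current speed.
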(event `self.ReceiveBeginPlay`
  (`KismetSystemLibrary.K2_SetTimer` null "CheckForDoorsToOpen" 1.5 true))

(event `self.ReceiveTick`
  (params (DeltaSeconds :type "Float (single-precision)"))
  (bind _charactermovement (`self.CharacterMovement`))
  (bind _returnvalue (`KismetMathLibrary.MapRangeClamped` (`self.ScaleSprite`) 0.0 50.0 0.0 (`CharacterMovementComponent.MaxWalkSpeed` _charactermovement)))
  ;[1 1 1] Intended to scale the sprint larger for faster movement on motion tracker
  (if (> (`KismetMathLibrary.VSize` (`MovementComponent.Velocity` _charactermovement)) 0.0)
    (`SceneComponent.SetWorldScale3D` (`self.PaperSprite`) (`KismetMathLibrary.MakeVector` _returnvalue _returnvalue _returnvalue))
    (else
      (`SceneComponent.SetWorldScale3D` (`self.PaperSprite`) (0.0 0.0 0.0)))))

(fn `CheckForDoorsToOpen`
  (bind _returnvalue (`self.K2_GetActorLocation`))
  (bind _outhit (`KismetSystemLibrary.LineTraceSingle` _returnvalue (+ _returnvalue (* (`self.GetActorForwardVector`) 50.0)) "TraceTypeQuery1"))
  (bind _asbp_interact_door (cast `/Game/Environment/Doors/BP_InteractDoor` (`.HitActor` (`GameplayStatics.BreakHitResult` _outhit))))
  (message `/Game/Blueprints/Interfaces/BPI_Interact.Interact` _asbp_interact_door "/Script/GunsOfDinosaurs.MonsterCharacter"))

(fn `UserConstructionScript`)