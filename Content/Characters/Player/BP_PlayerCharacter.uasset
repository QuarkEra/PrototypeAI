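; First-person player character with three weapon slots, flashlight, flares, crouch and interaction.
; Weapons attach to Mesh1P, either spawned from the game instance's backpack or equipped into the first free slot, and switch through visibility and active flags.
; Hard-wired keys drive the actions and debug speed changes, with interaction using a camera trace and BPI_Interact.
; Tick scales a Paper sprite for the motion tracker, collapsing it when stationary.
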(event `self.ReceiveTick`
  (params (DeltaSeconds :type "Float (single-precision)"))
  (bind _charactermovement (`self.CharacterMovement`))
  (bind _returnvalue (`KismetMathLibrary.MapRangeClamped` (`self.ScaleSprite`) 0.0 25.0 0.0 (`CharacterMovementComponent.MaxWalkSpeed` _charactermovement)))
  ;[1 1 1] Intended to scale the sprint larger for faster movement on motion tracker
  (if (> (`KismetMathLibrary.VSize` (`MovementComponent.Velocity` _charactermovement)) 0.0)
    (`SceneComponent.SetWorldScale3D` (`self.PaperSprite`) (`KismetMathLibrary.MakeVector` _returnvalue 0.0 _returnvalue))
    (else
      (`SceneComponent.SetWorldScale3D` (`self.PaperSprite`) (0.0 0.0 0.0)))))

(event `Key|One`
  (params (Key :type "Key Structure"))
  (bind _charactermovement (`self.CharacterMovement`))
  ;[1 1 1] Debug
  (:`Pressed`
    (set `CharacterMovementComponent.MaxWalkSpeed` (+ (`CharacterMovementComponent.MaxWalkSpeed` _charactermovement) 500.0) _charactermovement)))

(event `Key|Two`
  (params (Key :type "Key Structure"))
  (bind _charactermovement (`self.CharacterMovement`))
  ;[1 1 1] Debug
  (:`Pressed`
    (set `CharacterMovementComponent.MaxWalkSpeed` (- (`CharacterMovementComponent.MaxWalkSpeed` _charactermovement) 500.0) _charactermovement)))

(event `Key|T`
  (params (Key :type "Key Structure"))
  (bind (_returnvalue_roll _returnvalue_pitch _returnvalue_yaw) (`KismetMathLibrary.BreakRotator` (`KismetMathLibrary.MakeRotFromX` (`SceneComponent.GetForwardVector` (`self.CameraComp`)))))
  (:`Pressed`
    (`|SpawnActorFromClass` "/Game/Blueprints/BP_Flare.BP_Flare_C" (`KismetMathLibrary.MakeTransform` (`SceneComponent.GetSocketLocation` (`self.Mesh1P`) "GripPoint") (`KismetMathLibrary.MakeRotator` _returnvalue_roll (+ _returnvalue_pitch 25.0) _returnvalue_yaw)) "AdjustIfPossibleButAlwaysSpawn" "MultiplyWithRoot" null null)))

(event `Key|SpaceBar`
  (params (Key :type "Key Structure"))
  (:`Pressed`
    (if (`NavMovementComponent.IsCrouching` (`self.CharacterMovement`))
      (`self.UnCrouch`)
      (else
        (`self.Crouch`)))))

(event `Key|R`
  (params (Key :type "Key Structure"))
  ;[1 1 1] Reveal Weapon
  (:`Pressed`
    (bind _currentweapon (`self.CurrentWeapon`)
      (:`then`
        (if true
          (if (`Actor.bHidden` _currentweapon)
            (`self.SetActorHiddenInGame` _currentweapon false)
            (set `GodWeapon.bIsActiveWeapon` true _currentweapon)
            (else
              (`self.SetActorHiddenInGame` _currentweapon true)
              (set `GodWeapon.bIsActiveWeapon` false _currentweapon)))))
      (:`else`))))

(event `Key|F`
  (params (Key :type "Key Structure"))
  (:`Pressed`
    (`SceneComponent.ToggleVisibility` (`self.SpotLight`) false)))

(event `Key|E`
  (params (Key :type "Key Structure"))
  (:`Pressed`
    (bind _hitactor (`self.LineTrace` (`self.TouchLength`)))
    (if (`KismetSystemLibrary.DoesImplementInterface` _hitactor "/Game/Blueprints/Interfaces/BPI_Interact.BPI_Interact_C")
      (message `/Game/Blueprints/Interfaces/BPI_Interact.Interact` _hitactor "BP_PlayerCharacter_C"))))

(fn `EquipWeapon`
  (params (NewWeapon :type "/Game/Weapons/Common/BP_WeaponBase Class Reference"))
  (bind _newlyspawnedweapon (`self.NewlySpawnedWeapon`))
  (bind _returnvalue (`|SpawnActorFromClass` NewWeapon (`SceneComponent.GetSocketTransform` (`self.Mesh1P`) (`self.SocketName`) "RTS_World") "AlwaysSpawn" "MultiplyWithRoot" null 0 true null))
  (bind _output_get (set `self.NewlySpawnedWeapon` _returnvalue))
  (`self.K2_AttachToComponent` _output_get (`self.Mesh1P`) (`self.SocketName`) "SnapToTarget" "SnapToTarget" "SnapToTarget" true)
  (`self.SetActorHiddenInGame` _output_get false)
  (bind _output_get_2 (set `self.CurrentWeapon` _output_get))
  (set `GodWeapon.bIsCollected` true _output_get_2)
  (`GameplayStatics.SpawnSound2D` "/Game/Audio/CC-DS_Whoosh_Leather_Hard_01_Cue.CC-DS_Whoosh_Leather_Hard_01_Cue" 1.0 1.0 0.0 null)
  (`/Engine/EditorBlueprintResources/StandardMacros.IsValid` (`self.WeaponSlot1`)
    (:`Is Valid`
      (`/Engine/EditorBlueprintResources/StandardMacros.IsValid` (`self.WeaponSlot2`)
        (:`Is Valid`
          (`/Engine/EditorBlueprintResources/StandardMacros.IsValid` (`self.WeaponSlot3`)
            (:`Is Not Valid`
              (bind _output_get_3 (set `self.WeaponSlot3` _newlyspawnedweapon))
              (`self.Set Current Weapon` _output_get_3 _newlyspawnedweapon))))
        (:`Is Not Valid`
          (bind _output_get_4 (set `self.WeaponSlot2` (`self.NewlySpawnedWeapon`)))
          (`self.Set Current Weapon` _output_get_4 (`self.NewlySpawnedWeapon`)))))
    (:`Is Not Valid`
      (bind _output_get_5 (set `self.WeaponSlot1` (`self.NewlySpawnedWeapon`)))
      (`self.Set Current Weapon` _output_get_5 (`self.NewlySpawnedWeapon`)))))

(fn `InstantiateWeapons`
  (bind _asbp_gi_guns_of_dinosaurs (cast `/Game/Core/BP_GI_GunsOfDinosaurs` (`GameplayStatics.GetGameInstance`)))
  (for (_array_element _array_index) (`/Game/Core/BP_GI_GunsOfDinosaurs.BackpackWeapons` _asbp_gi_guns_of_dinosaurs)
    (bind _returnvalue (`|SpawnActorFromClass` (`.WeaponToSpawn_24_F699F5BC45CC16F5A56A9191A0C819D0` (break `/Game/Core/FWeaponBackpack` _array_element)) (`SceneComponent.GetSocketTransform` (`self.Mesh1P`) "GripPoint" "RTS_World") "AlwaysSpawn" "MultiplyWithRoot" null _array_index false null))
    (bind _returnvalue_2 (`self.K2_AttachToComponent` _returnvalue (`self.Mesh1P`) "GripPoint" "SnapToTarget" "SnapToTarget" "SnapToTarget" true))
    (`self.SetActorHiddenInGame` _returnvalue _returnvalue_2)
    (switch `int` _array_index
      (:`0`
        (set `self.WeaponSlot1` _returnvalue))
      (:`1`
        (set `self.WeaponSlot2` _returnvalue))
      (:`2`
        (set `self.WeaponSlot3` _returnvalue)))))

(fn `LineTrace`
  (params (Length :type "Float (double-precision)" :default 350.0))
  (returns (HitActor :type "Actor Object Reference"))
  (bind _cameracomp (`self.CameraComp`))
  (bind _returnvalue (`SceneComponent.K2_GetComponentLocation` _cameracomp))
  (bind _outhit (`KismetSystemLibrary.LineTraceSingle` _returnvalue (+ _returnvalue (* (`SceneComponent.GetForwardVector` _cameracomp) Length)) "TraceTypeQuery1"))
  (return (`.HitActor` (`GameplayStatics.BreakHitResult` _outhit))))

(fn `Set Current Weapon`
  (params (WeaponSlot :type "/Game/Weapons/Common/BP_WeaponBase Object Reference") (NewWeapon :type "/Game/Weapons/Common/BP_WeaponBase Object Reference"))
  (bind _currentweapon (`self.CurrentWeapon`))
  (if (`GodWeapon.bIsCollected` NewWeapon)
    (if (!= WeaponSlot _currentweapon)
      (set `GodWeapon.bIsActiveWeapon` false _currentweapon)
      (`self.SetActorHiddenInGame` _currentweapon true)
      (`self.SetActorHiddenInGame` WeaponSlot false)
      (bind _output_get (set `self.CurrentWeapon` WeaponSlot))
      (set `GodWeapon.bIsActiveWeapon` true _output_get))))

(fn `UserConstructionScript`)